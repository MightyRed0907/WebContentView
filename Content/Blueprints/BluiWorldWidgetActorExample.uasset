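; Example actor that shows a Blui web browser widget on the player's screen.
; On BeginPlay, if LoadOnStartup is set, InitBluiWidget creates the widget for the first player controller, which is then added to the viewport.
; Initialization passes the invalid-URL auto-search flag, BluEye settings and default URL from the actor's variables to the widget.
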(event EventBeginPlay
  (if (Variables|Default|GetLoadOnStartup)
    (CallFunction|InitBluiWidget)
    (UserInterface|Viewport|AddtoViewport (Variables|Default|GetBluiWidget) 0)))

(event Collision|EventActorBeginOverlap
  (params (OtherActor :type Actor%20Object%20Reference)))

(event EventTick
  (params (DeltaSeconds :type Float%20%28single-precision%29)))

(fn ConstructionScript)

(fn InitBluiWidget
  (bind _returnvalue (UserInterface|CreateWidget "/Game/Blueprints/BluiWidget.BluiWidget_C" (Game|GetPlayerController 0)))
  (bind _output_get (Variables|Default|SetBluiWidget _returnvalue))
  (Variables|/Game/Blueprints/BluiWidget.BluiWidget_C|SetShouldAutoSearch _output_get (Variables|Default|GetShouldAutoSearchInvalidUrl))
  (Default|InitBluEye (Variables|Default|GetBluiWidget) (Variables|Default|GetInitBluEyeSettings) (Variables|Default|GetUrl)))